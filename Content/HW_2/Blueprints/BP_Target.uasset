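; BP_Target is a shootable target that tracks Health and counts toward the player's score of targets hit.
; Its Hit event reacts only to BP_ShooterProjectileBase actors, subtracting a fixed amount of Health per hit.
; When Health drops below one, it increments TargetsHit on player 0's BP_ShooterCharacter and destroys itself.
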(event `self.ReceiveHit`
  (params (MyComp :type "PrimitiveComponent Object Reference") (Other :type "Actor Object Reference") (OtherComp :type "PrimitiveComponent Object Reference") (bSelfMoved :type Boolean) (HitLocation :type "Vector Structure") (HitNormal :type "Vector Structure") (NormalImpulse :type "Vector Structure") (Hit :type "HitResult Structure (by ref)"))
  (bind _health (`self.health`))
  (cast `/Game/Variant_Shooter/Blueprints/Pickups/Projectiles/BP_ShooterProjectileBase` Other)
  (bind _asbp_shooter_character (cast `/Game/Variant_Shooter/Blueprints/BP_ShooterCharacter` (`GameplayStatics.GetPlayerCharacter` 0)))
  (set `self.health` (- _health 25))
  (if (< _health 1)
    (set `/Game/Variant_Shooter/Blueprints/BP_ShooterCharacter.Targets_Hit` (+ (`/Game/Variant_Shooter/Blueprints/BP_ShooterCharacter.Targets_Hit` _asbp_shooter_character) 1) _asbp_shooter_character)
    (`self.K2_DestroyActor`)))

(fn `UserConstructionScript`)